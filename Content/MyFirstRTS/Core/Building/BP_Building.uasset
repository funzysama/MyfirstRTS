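; BP_Building is a building actor that the player can select by clicking in an RTS.
; A click fires BuildingClickedEvent, which adds the building to the selected list on PC_MyFirstRTS and reveals its Decal as a selection indicator.
; DeselectThis hides the Decal again, leaving the controller's list untouched.
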(event Custom|BuildingClickedEvent
  (bind _decal (Variables|Default|GetDecal))
  (Utilities|FlowControl|Sequence
    (:then_0
      (bind _aspc_my_first_rts (Utilities|Casting|CastToPC_MyFirstRTS (Game|GetPlayerController 0)))
      (Default|AddActortoSelectedList _aspc_my_first_rts self))
    (:then_1
      (Development|SetHiddeninGame _decal false false)
      (Rendering|SetVisibility _decal true false))))

(event EventBeginPlay)

(event Collision|EventActorBeginOverlap
  (params (OtherActor :type Actor%20Object%20Reference)))

(event EventTick
  (params (DeltaSeconds :type Float%20%28single-precision%29)))

(event MouseInput|EventActorOnClicked
  (params (ButtonPressed :type Key%20Structure :default "None"))
  (CallFunction|BuildingClickedEvent))

(event EventDeselectThis
  (bind _decal (Variables|Default|GetDecal))
  (Development|SetHiddeninGame _decal true false)
  (Rendering|SetVisibility _decal false false))

(fn ConstructionScript)