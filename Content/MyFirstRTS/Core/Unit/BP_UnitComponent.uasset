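; BP_UnitComponent is an RTS component that makes its owning actor selectable by clicking.
; On BeginPlay it binds a handler to the owner's OnClicked event.
; A click adds the owner to the selected list on PC_MyFirstRTS and reveals the owner's DecalComponent as a selection marker.
; It only handles selecting, with no logic to deselect or hide the decal.
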(event Custom|OnOwnerClicked
  (params (TouchedActor :type Actor%20Object%20Reference) (ButtonPressed :type Key%20Structure :default "None"))
  (CallFunction|AddUnittoSelectionList)
  (CallFunction|ShowSelectionDecal))

(event Custom|ShowSelectionDecal
  (bind _returnvalue (Components|GetOwner))
  (bind _returnvalue_2 (Actor|GetComponentbyClass _returnvalue "/Script/Engine.DecalComponent"))
  (Development|SetHiddeninGame _returnvalue_2 false false)
  (Rendering|SetVisibility _returnvalue_2 true false))

(event Custom|AddUnitToSelectionList
  (bind _aspc_my_first_rts (Utilities|Casting|CastToPC_MyFirstRTS (Game|GetPlayerController 0)))
  (Default|AddActortoSelectedList _aspc_my_first_rts (Components|GetOwner)))

(event EventBeginPlay
  (EventDispatchers|BindEventtoOnClicked (Components|GetOwner) (EventDispatchers|CreateEvent :!event Custom|OnOwnerClicked)))

(event EventTick
  (params (DeltaSeconds :type Float%20%28single-precision%29)))